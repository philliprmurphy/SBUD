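; Asteroid actor that spins in space and damages the player on collision.
; On BeginPlay it takes a random rotation and angular impulse, and the MenuAsteroid flag clears its lifespan so it does not expire.
; Hitting an actor tagged Player calls TakeDamage on the God actor found by class, plays an explosion sound at random pitch, and destroys the asteroid.
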(event EventBeginPlay
  (Transformation|SetActorRotation (Math|Random|RandomRotator false))
  (Class|PrimitiveComponent|AddAngularImpulseinRadians (Variables|Debug|GetStaticMeshComponent) (Math|Random|RandomUnitVector) "None" true)
  (if (Variables|Default|GetmenuAsteroid)
    (Actor|SetLifeSpan 0.0)))

(event Collision|EventHit
  (params (MyComp :type Primitive%20Component%20Object%20Reference) (Other :type Actor%20Object%20Reference) (OtherComp :type Primitive%20Component%20Object%20Reference) (bSelfMoved :type Boolean) (HitLocation :type Vector :default "0, 0, 0") (HitNormal :type Vector :default "0, 0, 0") (NormalImpulse :type Vector :default "0, 0, 0") (Hit :type Hit%20Result%20Structure%20%28by%20ref%29))
  (if (Actor|ActorHasTag Other "Player")
    (bind _returnvalue (Actor|GetActorOfClass "/Game/MyContent/Blueprints/God.God_C"))
    (Default|TakeDamage _returnvalue)
    (Audio|PlaySound2D "/Game/StarterContent/Audio/Explosion_Cue.Explosion_Cue" 0.5 (Math|Random|RandomFloatinRange 0.5 1.5) 0.0 0 0)
    (Actor|DestroyActor)))

(fn ConstructionScript)
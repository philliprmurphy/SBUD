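; God is the game manager for an obstacle-dodging spaceship game, handling HUD, scoring, money, hit points and obstacle spawning.
; At play outside menus, it applies Game Instance difficulty and bonus HP, then starts a delayed self-repeating money and score tick.
; SpawnObs builds dodge patterns through SpawnAhead, which places obstacles by lead time and song speed and sets their physics velocity.
; TakeDamage respects god mode, penalizes score, and at zero HP stops the LevelSequence and shows the Lose screen.
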(event Custom|IncrementMoneyScore
  (if (not (Variables|Default|Getpaused))
    (bind _asspace_game_instance (Utilities|Casting|CastToSpaceGameInstance (Game|GetGameInstance)))
    (Variables|/Game/MyContent/Blueprints/SpaceGameInstance.SpaceGameInstance_C|Setmoney _asspace_game_instance (+ (Variables|/Game/MyContent/Blueprints/SpaceGameInstance.SpaceGameInstance_C|Getmoney _asspace_game_instance) 100))
    (Variables|Default|SetcurrScore (+ (Variables|Default|GetcurrScore) (Math|Float|Truncate (* 2000 (Variables|/Game/MyContent/Blueprints/SpaceGameInstance.SpaceGameInstance_C|Getdifficulty _asspace_game_instance)))))
    (Default|UpdateMoneyScore (Variables|Default|GetGUI))
    (Utilities|FlowControl|Delay 2.0)
    (CallFunction|IncrementMoneyScore)))

(event EventBeginPlay
  (if (not (Variables|Default|GetinMenu))
    (bind _returnvalue (Actor|GetActorOfClass "/Game/MyContent/Blueprints/PlayerShip.PlayerShip_C"))
    (Variables|Default|Setship _returnvalue)
    (bind _asspace_game_instance (Utilities|Casting|CastToSpaceGameInstance (Game|GetGameInstance)))
    (Variables|Default|SetobsSpeedMulti (* (Variables|/Game/MyContent/Blueprints/SpaceGameInstance.SpaceGameInstance_C|Getdifficulty _asspace_game_instance) (Variables|Default|GetobsSpeedMulti)))
    (bind _output_get (Variables|Default|SethitPoints (+ (Variables|/Game/MyContent/Blueprints/SpaceGameInstance.SpaceGameInstance_C|GetbonusHP _asspace_game_instance) (Variables|Default|GethitPoints))))
    (Variables|Default|SetmaxHP _output_get)
    (bind _returnvalue_2 (UserInterface|CreateWidget "/Game/MyContent/Widgets/GUI.GUI_C"))
    (bind _output_get_2 (Variables|Default|SetGUI _returnvalue_2))
    (UserInterface|Viewport|AddtoViewport _output_get_2 0)
    (Utilities|FlowControl|Delay 3.0)
    (CallFunction|IncrementMoneyScore)))

(fn ConstructionScript)

(fn SpawnAhead
  (params (secondsAhead :type Float%20%28single-precision%29) (obsIndex :type Integer) (Yoffset :type Float%20%28single-precision%29) (Zoffset :type Float%20%28single-precision%29))
  (bind _output_get (Variables|Default|SetobsSpeed (* (Variables|Default|GetcurrSongSpeed) (Variables|Default|GetobsSpeedMulti))))
  (bind _returnvalue (Game|SpawnActorfromClass (Utilities|Array|Get(acopy) (Variables|Default|GetobsArray) obsIndex) (Math|Transform|MakeTransform (Math|Vector|MakeVector (+ (.x (Transformation|GetWorldLocation (Variables|/Game/MyContent/Blueprints/PlayerShip.PlayerShip_C|GetSciFi_Fighter (Variables|Default|Getship)))) (* _output_get secondsAhead)) Yoffset (+ Zoffset 2e+02)) "0, 0, 0" "1,1,1") "Undefined" 0 0))
  (bind _result (Math|Float|NegateFloat (Variables|Default|GetobsSpeed))
    (:%20%20
      (Physics|SetPhysicsLinearVelocity (Actor|GetComponentbyClass _returnvalue "/Script/Engine.StaticMeshComponent") (Math|Vector|MakeVector _result 0.0 0.0) false "None"))))

(fn PauseGame
  (Class|MovieSceneSequencePlayer|StopatCurrentTime (Variables|/Script/LevelSequence.LevelSequenceActor|GetSequencePlayer (Variables|Default|GetlevelSequence)))
  (Variables|/Script/Engine.PlayerController|SetbShowMouseCursor (Game|GetPlayerController 0) true)
  (Variables|Default|Setpaused true))

(fn TakeDamage
  (bind _gui (Variables|Default|GetGUI))
  (bind _asspace_game_instance (Utilities|Casting|CastToSpaceGameInstance (Game|GetGameInstance)))
  (if (not (Variables|/Game/MyContent/Blueprints/SpaceGameInstance.SpaceGameInstance_C|GetgodModeEnabled _asspace_game_instance))
    (bind _result (Math|Integer|DecrementInt (Variables|Default|GethitPoints))
      (:%20%20
        ;[1 1 1] GUI/Money/Score Updates
        (Variables|Default|SetcurrScore (- (Variables|Default|GetcurrScore) (Variables|Default|GetscoreDmgPenalty)))
        (Default|UpdateMoneyScore _gui)
        (Default|UpdateHitPoints _gui)
        (if (and (not (Variables|Default|Getpaused)) (< _result 1))
          (CallFunction|PauseGame)
          (bind _returnvalue (UserInterface|CreateWidget "/Game/MyContent/Widgets/Lose.Lose_C"))
          (UserInterface|Viewport|AddtoViewport _returnvalue 0)
          (Input|SetInputModeUIOnly (Game|GetPlayerController 0) _returnvalue "DoNotLock"))))))

(fn SpawnObs
  (params (obstacle :type String) (secondAhead :type Float%20%28single-precision%29))
  (switch string obstacle
    (:Default
      ;[1 1 1] Default
      (CallFunction|SpawnAhead secondAhead 0 0.0 0.0 :!label _label))
    (:sides
      ;[1 1 1] All Sides
      (CallFunction|SpawnAhead secondAhead 0 -4e+02 0.0)
      (CallFunction|SpawnAhead secondAhead 0 4e+02 0.0)
      (CallFunction|SpawnAhead secondAhead 0 0.0 4e+02))
    (:dodge%20left
      ;[1 1 1] Dodge left
      (CallFunction|SpawnAhead secondAhead 0 4e+02 0.0)
      (CallFunction|SpawnAhead secondAhead 0 0.0 4e+02)
      (goto _label))
    (:dodge%20right
      ;[1 1 1] Dodge right
      (CallFunction|SpawnAhead secondAhead 0 -4e+02 0.0)
      (CallFunction|SpawnAhead secondAhead 0 0.0 4e+02)
      (goto _label))
    (:dodge%20up
      ;[1 1 1] Dodge up
      (CallFunction|SpawnAhead secondAhead 0 4e+02 0.0)
      (CallFunction|SpawnAhead secondAhead 0 -4e+02 0.0)
      (goto _label))))
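; Player ship pawn that possesses itself on BeginPlay and dodges left, right or up, or rams forward, from a fixed start position.
; Dodge sets physics velocity on the SciFiFighter until DodgeDelay expires or a dodge key is released.
; DodgeCancel reverses the velocity for a distance-over-speed delay, then stops and snaps the ship home as a failsafe.
; IsMoving and Returning guard against overlapping moves; fire and shield inputs are empty stubs.
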(event Custom|Dodge
  (params (dodgeVec :type Vector :default "0,0.000000,0"))
  (Variables|Default|SetisMoving true)
  (Physics|SetPhysicsLinearVelocity (Variables|Default|GetSciFi_Fighter) dodgeVec false "None")
  (Utilities|FlowControl|Delay (Variables|Default|GetdodgeDelay))
  (if (Variables|Default|GetisMoving)
    (CallFunction|DodgeCancel dodgeVec)))

(event Custom|DodgeCancel
  (params (dodgeVec :type Vector))
  (bind _scifi_fighter (Variables|Default|GetSciFi_Fighter))
  (if (not (Variables|Default|Getreturning))
    (Variables|Default|Setreturning true)
    (Physics|SetPhysicsLinearVelocity _scifi_fighter (Math|Vector|NegateVector dodgeVec) false "None")
    (Utilities|FlowControl|Delay (/ (Math|Vector|VectorLength (- (Transformation|GetWorldLocation _scifi_fighter) (Variables|Default|GetstartLoc))) (Math|Vector|VectorLength dodgeVec)))
    (Physics|SetPhysicsLinearVelocity _scifi_fighter "0, 0, 0" false "None")
    (Variables|Default|SetisMoving false)
    (Variables|Default|Setreturning false)
    ;[1 1 1] Failsafe
    (Transformation|SetWorldLocation (Variables|Default|GetSciFi_Fighter) (Variables|Default|GetstartLoc) true true)))

(event EventBeginPlay
  (bind _returnvalue (Game|GetPlayerController 0))
  (Pawn|Possess (Game|GetPlayerController 0))
  (Variables|Default|SetstartLoc (Transformation|GetWorldLocation (Variables|Default|GetSciFi_Fighter)))
  (Input|SetInputModeGameOnly _returnvalue)
  (Variables|/Script/Engine.PlayerController|SetbShowMouseCursor _returnvalue false))

(event Input|ActionEvents|InputActiondodgeLeft
  (params (Key :type Key%20Structure :default "None"))
  (bind _ismoving (Variables|Default|GetisMoving))
  (bind _velocitymulti (Variables|Default|GetvelocityMulti))
  (bind _returnvalue (* -1 _velocitymulti))
  (:Pressed
    (if (not _ismoving)
      (CallFunction|Dodge (Math|Vector|MakeVector 0.0 _returnvalue 0.0))))
  (:Released
    (if _ismoving
      (CallFunction|DodgeCancel (Math|Vector|MakeVector 0.0 _returnvalue 0.0)))))

(event Input|ActionEvents|InputActiondodgeRight
  (params (Key :type Key%20Structure :default "None"))
  (bind _ismoving (Variables|Default|GetisMoving))
  (bind _velocitymulti (Variables|Default|GetvelocityMulti))
  (:Pressed
    (if (not _ismoving)
      (CallFunction|Dodge (Math|Vector|MakeVector 0.0 _velocitymulti 0.0))))
  (:Released
    (if _ismoving
      (CallFunction|DodgeCancel (Math|Vector|MakeVector 0.0 _velocitymulti 0.0)))))

(event Input|ActionEvents|InputActiondodgeUp
  (params (Key :type Key%20Structure :default "None"))
  (bind _velocitymulti (Variables|Default|GetvelocityMulti))
  (:Pressed
    (if (not (Variables|Default|GetisMoving))
      (CallFunction|Dodge (Math|Vector|MakeVector 0.0 0.0 _velocitymulti))))
  (:Released
    (if true
      (CallFunction|DodgeCancel (Math|Vector|MakeVector 0.0 0.0 _velocitymulti)))))

(event Input|ActionEvents|InputActionram
  (params (Key :type Key%20Structure :default "None"))
  (:Pressed
    (if (not (Variables|Default|GetisMoving))
      (CallFunction|Dodge (Math|Vector|MakeVector (Variables|Default|GetvelocityMulti) 0.0 0.0)))))

(event Input|ActionEvents|InputActionfire
  (params (Key :type Key%20Structure :default "None"))
  (:Pressed
    (if (Variables|Default|GetisMoving)
      _)))

(event Input|ActionEvents|InputActionshield
  (params (Key :type Key%20Structure :default "None"))
  (:Pressed
    (if (Variables|Default|GetisMoving)
      _)))

(fn ConstructionScript)
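; PoobleBP is an AI pawn that wanders around the navmesh on its own.
; From BeginPlay it loops: a random delay of a few seconds, then an AI move to a random navigable point near its current location.
; Success and failure both restart the loop, which only continues while the Partying flag is false.
; Nothing in this graph sets Partying or restarts wandering once it stops.
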(event Custom|randomMovement
  (if (not (Variables|Default|Getpartying))
    (Utilities|FlowControl|Delay (Math|Random|RandomFloatinRange 0.0 5.0))
    (AI|AIMoveTo self (.RandomLocation (Class|NavigationSystemV1|GetRandomPointinNavigableRadius (Transformation|GetActorLocation) 8e+02 0 0)) 0 5.0 false
      (:OnSuccess
        _)
      (:OnFail
        _))
    (CallFunction|RandomMovement)))

(event EventBeginPlay
  (CallFunction|RandomMovement))

(event EventTick
  (params (DeltaSeconds :type Float%20%28single-precision%29)))

(fn ConstructionScript)